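; Actor that displays a hand of cards, called pages, in a card game as an animated fan.
; On BeginPlay it spawns a BP_PageVisual per starting page, then computes centered, angled target offsets in the hand's local space.
; Targets are stored in per-page position and rotation maps.
; Tick interpolates pages toward those targets and removes each map entry once it is reached.
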(event EventBeginPlay
  (CallFunction|SpawnPages)
  (CallFunction|SpacialDistribute))

(event Collision|EventActorBeginOverlap
  (params (OtherActor :type Actor%20Object%20Reference)))

(event EventTick
  (params (DeltaSeconds :type Float%20%28single-precision%29))
  (Variables|Default|SetDelta%20Seconds DeltaSeconds)
  (CallFunction|UpdatePagesDistribution))

(fn ConstructionScript)

(fn SpawnPages
  (Variables|Default|SetSelectedPage 0)
  (Utilities|Array|Clear (Variables|Default|GetPages))
  (for _array_element (Variables|Params|GetHandStartingPages)
    (bind _returnvalue (Game|SpawnActorfromClass "/Game/CardTest/BP_PageVisual.BP_PageVisual_C" (Transformation|GetActorTransform) "Undefined" "MultiplyWithRoot" 0 _array_element 0))
    (Utilities|Array|Add (Variables|Default|GetPages) _returnvalue))
  (return))

(fn SpacialDistribute
  (bind _distributionspacing (Variables|Params|GetDistributionSpacing))
  (Utilities|Map|Clear (Variables|Default|GetDesiredPositionsMap))
  (Utilities|Map|Clear (Variables|Default|GetDesiredRotationsMap))
  (if (Utilities|Array|IsEmpty (Variables|Default|GetPages))
    (return)
    (else
      (LocalVariables|SetPageCount (Utilities|Array|Length (Variables|Default|GetPages)))
      (for (_array_element _array_index) (Variables|Default|GetPages)
        (LocalVariables|SetCurrentPage _array_element)
        (LocalVariables|SetPageIndex _array_index)
        (LocalVariables|SetCurrentSpatialModifier (/ (- (* (LocalVariables|GetPageIndex) 2) (- (LocalVariables|GetPageCount) 1)) 2.0))
        (Utilities|Map|Add (Variables|Default|GetDesiredPositionsMap) (LocalVariables|GetCurrentPage) (+ (Transformation|GetActorLocation (LocalVariables|GetCurrentPage)) (Math|Transform|TransformDirection (Transformation|GetActorTransform) (Math|Vector|MakeVector (* (LocalVariables|GetCurrentSpatialModifier) (.x _distributionspacing)) (* (.y _distributionspacing) (LocalVariables|GetPageIndex)) (* (Math|Float|Absolute(Float) (Math|Trig|Tan(Degrees) (* (LocalVariables|GetCurrentSpatialModifier) (Variables|Params|GetDistributionAngle)))) (* (.x (Variables|Params|GetDistributionSpacing)) -2.0))))))
        (Utilities|Map|Add (Variables|Default|GetDesiredRotationsMap) (LocalVariables|GetCurrentPage) (Math|Transform|TransformRotation (Transformation|GetActorTransform) (Math|Rotator|MakeRotator 0.0 (* (LocalVariables|GetCurrentSpatialModifier) (Variables|Params|GetDistributionAngle)) 0.0))))
      (return))))

(fn UpdatePagesDistribution
  (Utilities|FlowControl|Sequence
    (:then_0
      (bind _keys (Utilities|Map|Keys (Variables|Default|GetDesiredPositionsMap)))
      (for _array_element _keys
        (LocalVariables|SetCurrentPage _array_element)
        (LocalVariables|SetCurrentPosition (Transformation|GetActorLocation (LocalVariables|GetCurrentPage)))
        (if (.ReturnValue (Utilities|Map|Find (Variables|Default|GetDesiredPositionsMap) (LocalVariables|GetCurrentPage)))
          (LocalVariables|SetCurrentDesiredPosition (.Value (Utilities|Map|Find (Variables|Default|GetDesiredPositionsMap) (LocalVariables|GetCurrentPage))))
          (if (Utilities|Operators|EqualEqual (LocalVariables|GetCurrentPosition) (LocalVariables|GetCurrentDesiredPosition) 0.01)
            (Utilities|Map|Remove (Variables|Default|GetDesiredPositionsMap) (LocalVariables|GetCurrentPage))
            (else
              (Transformation|SetActorLocation (LocalVariables|GetCurrentPage) (Math|Interpolation|VInterpTo (LocalVariables|GetCurrentPosition) (LocalVariables|GetCurrentDesiredPosition) (Variables|Default|GetDelta%20Seconds) (Variables|Params|GetDistributionSpeed)) false false))))))
    (:then_1
      (bind _keys_2 (Utilities|Map|Keys (Variables|Default|GetDesiredRotationsMap)))
      (for _array_element_2 _keys_2
        (LocalVariables|SetCurrentPage _array_element_2)
        (LocalVariables|SetCurrentRotation (Transformation|GetActorRotation (LocalVariables|GetCurrentPage)))
        (if (.ReturnValue (Utilities|Map|Find (Variables|Default|GetDesiredRotationsMap) (LocalVariables|GetCurrentPage)))
          (LocalVariables|SetCurrentDesiredRotation (.Value (Utilities|Map|Find (Variables|Default|GetDesiredRotationsMap) (LocalVariables|GetCurrentPage))))
          (if (Utilities|Operators|EqualEqual (LocalVariables|GetCurrentRotation) (LocalVariables|GetCurrentDesiredRotation) 0.01)
            (Utilities|Map|Remove (Variables|Default|GetDesiredRotationsMap) (LocalVariables|GetCurrentPage))
            (else
              (Transformation|SetActorRotation (LocalVariables|GetCurrentPage) (Math|Interpolation|RInterpTo (LocalVariables|GetCurrentRotation) (LocalVariables|GetCurrentDesiredRotation) (Variables|Default|GetDelta%20Seconds) (Variables|Params|GetDistributionSpeed))))))))))