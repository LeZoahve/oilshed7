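; BP_SpellAnimation is a spell effect actor that repeatedly emits animated shapes between an origin and a target grid tile.
; From BeginPlay, a delay loop triggers the play-animation event several times per second.
; Each call spawns a yellow BP_AnimatedShape using the Grid's current shape mesh and material, passing both tile transforms as its start and end.
; The loop has no stop condition in this Blueprint.
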(event Custom|Event_PlaySpellAnimation
  (bind _grid (Variables|Default|GetGrid))
  (bind _returnvalue (Default|GetCurrentShapeData _grid))
  (bind _gridtiles (Variables|/Game/Blueprints/Core/Grid/BP_Grid.BP_Grid_C|GetGridTiles _grid))
  (Game|SpawnActorfromClass "/Game/Blueprints/Core/Spells/Components/BP_AnimatedShape.BP_AnimatedShape_C" (Math|Transform|MakeTransform "0, 0, 0" "0, 0, 0" "1.000000,1.000000,1.000000") "AlwaysSpawn" "MultiplyWithRoot" 0 (.mesh _returnvalue) (.meshmaterial _returnvalue) "(R=1.000000,G=1.000000,B=0.000000,A=1.000000)" (.transform (.Value (Utilities|Map|Find _gridtiles (Variables|Default|GetOriginIndex)))) (.transform (.Value (Utilities|Map|Find _gridtiles (Variables|Default|GetTargetIndex)))) 0))

(event EventBeginPlay
  (CallFunction|EventPlaySpellAnimation :!label _label)
  (Utilities|FlowControl|RetriggerableDelay 0.2)
  (goto _label))

(fn ConstructionScript)