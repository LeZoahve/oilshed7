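; BP_PlayerController is the player controller that sets up cursor input and player state when play begins.
; On BeginPlay it shows the mouse cursor, casts its PlayerState to BP_PlayerState and calls Init on it.
; A test event casts the current grimoire book spell through GrimoiresGameLogic, then prints the player state's HP for debugging.
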(event Custom|TESTEUH
  (Class|GrimoiresGameLogicComponent|CastCurrentBookSpell (Variables|Default|GetGrimoiresGameLogic))
  ;[1 1 1] Display
  (bind _asbp_player_state (Utilities|Casting|CastToBP_PlayerState (Variables|GetPlayerState self)))
  (Development|PrintString (Utilities|String|Append "HP : " (Utilities|String|ToString(Integer) (Variables|/Script/oilshed7.GrimoiresPlayerState|GetHP _asbp_player_state)))))

(event EventBeginPlay
  (Variables|Default|SetbShowMouseCursor true)
  (bind _asbp_player_state (Utilities|Casting|CastToBP_PlayerState (Variables|GetPlayerState self)))
  (Default|Init _asbp_player_state))

(fn ConstructionScript)