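; BP_Pawn is a player camera pawn that pans along world X/Y and zooms through Enhanced Input.
; BeginPlay adds IMC_Default, and input actions adjust a desired location and a clamped desired spring arm length.
; Tick eases the actor location and arm length toward those targets with interpolation, moving without sweep.
; The construction script seeds both targets from the current transform location and arm length.
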(event Input|EnhancedActionEvents|EnhancedInputActionIA_ZoomInOut
  (params (ActionValue :type Float%20%28double-precision%29) (ElapsedSeconds :type Float%20%28double-precision%29) (TriggeredSeconds :type Float%20%28double-precision%29) (InputAction :type Input%20Action%20Object%20Reference :default "/Game/Blueprints/Core/Inputs/IA_ZoomInOut.IA_ZoomInOut"))
  ;[1 1 1] Zoom Input to fDesiredCameraZoom
  (Variables|Default|SetfDesiredCameraZoom (Math|Float|Clamp(Float) (+ (Variables|Default|GetfDesiredCameraZoom) (* (Variables|Default|GetfZoomFactor) ActionValue)) 1e+02 5e+03)))

(event Input|EnhancedActionEvents|EnhancedInputActionIA_MoveLeft
  (params (ActionValue :type Float%20%28double-precision%29) (ElapsedSeconds :type Float%20%28double-precision%29) (TriggeredSeconds :type Float%20%28double-precision%29) (InputAction :type Input%20Action%20Object%20Reference :default "/Game/Blueprints/Core/Inputs/IA_MoveLeft.IA_MoveLeft"))
  ;[1 1 1] Move Input to fDesiredCameraLocation
  (Variables|Default|SetfDesiredCameraLocation (+ (Variables|Default|GetfDesiredCameraLocation) (Math|Vector|MakeVector 0.0 (* ActionValue (Variables|Default|GetfMoveSpeedFactor)) 0.0))))

(event Input|EnhancedActionEvents|EnhancedInputActionIA_MoveForward
  (params (ActionValue :type Float%20%28double-precision%29) (ElapsedSeconds :type Float%20%28double-precision%29) (TriggeredSeconds :type Float%20%28double-precision%29) (InputAction :type Input%20Action%20Object%20Reference :default "/Game/Blueprints/Core/Inputs/IA_MoveForward.IA_MoveForward"))
  ;[1 1 1] Move Input to fDesiredCameraLocation
  (Variables|Default|SetfDesiredCameraLocation (+ (Variables|Default|GetfDesiredCameraLocation) (Math|Vector|MakeVector (* ActionValue (Variables|Default|GetfMoveSpeedFactor)) 0.0 0.0))))

(event Input|EnhancedActionEvents|EnhancedInputActionIA_MoveBackward
  (params (ActionValue :type Float%20%28double-precision%29) (ElapsedSeconds :type Float%20%28double-precision%29) (TriggeredSeconds :type Float%20%28double-precision%29) (InputAction :type Input%20Action%20Object%20Reference :default "/Game/Blueprints/Core/Inputs/IA_MoveBackward.IA_MoveBackward"))
  ;[1 1 1] Move Input to fDesiredCameraLocation
  (Variables|Default|SetfDesiredCameraLocation (+ (Variables|Default|GetfDesiredCameraLocation) (Math|Vector|MakeVector (* ActionValue (Variables|Default|GetfMoveSpeedFactor)) 0.0 0.0))))

(event Input|EnhancedActionEvents|EnhancedInputActionIA_MoveRight
  (params (ActionValue :type Float%20%28double-precision%29) (ElapsedSeconds :type Float%20%28double-precision%29) (TriggeredSeconds :type Float%20%28double-precision%29) (InputAction :type Input%20Action%20Object%20Reference :default "/Game/Blueprints/Core/Inputs/IA_MoveRight.IA_MoveRight"))
  ;[1 1 1] Move Input to fDesiredCameraLocation
  (Variables|Default|SetfDesiredCameraLocation (+ (Variables|Default|GetfDesiredCameraLocation) (Math|Vector|MakeVector 0.0 (* ActionValue (Variables|Default|GetfMoveSpeedFactor)) 0.0))))

(event EventBeginPlay
  ;[1 1 1] Setup Mapping Context
  (bind _asplayer_controller (Utilities|Casting|CastToPlayerController (Pawn|GetController)))
  (Utilities|IsValid _asplayer_controller
    (:Is%20Valid
      (Input|AddMappingContext (PlayerController|LocalPlayerSubsystems|GetEnhancedInputLocalPlayerSubsystem _asplayer_controller) "/Game/Blueprints/Core/Inputs/IMC_Default.IMC_Default" 0 "(bIgnoreAllPressedKeysUntilRelease=True,bForceImmediately=False,bNotifyUserSettings=False)"))))

(event EventTick
  (params (DeltaSeconds :type Float%20%28single-precision%29))
  (bind _springarm (Variables|Default|GetSpringArm))
  ;[1 1 1] Interpolate fDesiredCameraZoom to SpringArmLength
  (Variables|/Script/Engine.SpringArmComponent|SetTargetArmLength _springarm (Math|Interpolation|FInterpTo (Variables|/Script/Engine.SpringArmComponent|GetTargetArmLength _springarm) (Variables|Default|GetfDesiredCameraZoom) DeltaSeconds 2.0))
  (Transformation|SetActorLocation (Math|Interpolation|VInterpTo (Transformation|GetActorLocation) (Variables|Default|GetfDesiredCameraLocation) DeltaSeconds 2.0) false false))

(fn ConstructionScript
  (CallFunction|InitVariables))

(fn InitVariables
  (Variables|Default|SetfDesiredCameraZoom (Variables|/Script/Engine.SpringArmComponent|GetTargetArmLength (Variables|Default|GetSpringArm)))
  (Variables|Default|SetfDesiredCameraLocation (Transformation|GetActorLocation)))