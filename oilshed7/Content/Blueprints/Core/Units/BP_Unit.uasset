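; BP_Unit is a unit Blueprint with Warrior and Ranger variants, currently set up to test unit animation states.
; The construction script picks the skeletal mesh and Animation Blueprint from UnitType.
; From BeginPlay, an endless three-second Delay loop cycles TestAnimState through six values and passes each to the anim instance through a SetUnitAnimationState message.
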(event EventBeginPlay
  (Utilities|FlowControl|Delay 3.0 :!label _label)
  (bind _output_get (Variables|Default|SetTestAnimState (Utilities|Enum|ByteToEnumE_UnitAnimState (Class|KismetMathLibrary|PercentByteByte (+ (Variables|Default|GetTestAnimState) 1) 6))))
  (Class|BPIUnitAnimation|SetUnitAnimationState(Message) (Components|SkeletalMesh|GetAnimInstance (Variables|Default|GetSkeletalMesh)) _output_get)
  (goto _label))

(fn ConstructionScript
  (bind _skeletalmesh (Variables|Default|GetSkeletalMesh))
  (bind _unittype (Variables|Default|GetUnitType))
  (Components|SkeletalMesh|SetSkeletalMeshAsset _skeletalmesh (Utilities|Select :Index _unittype :NewEnumerator0 "/Game/Art/Skeletons/Warrior/SK_Warrior.SK_Warrior" :NewEnumerator1 "/Game/Art/Skeletons/Ranger/SK_Ranger.SK_Ranger"))
  (Class|SkeletalMeshComponent|SetAnimClass _skeletalmesh (Utilities|Select :Index _unittype :NewEnumerator0 "/Game/Blueprints/Anim/ABP_Warrior.ABP_Warrior_C" :NewEnumerator1 "/Game/Blueprints/Anim/ABP_Ranger.ABP_Ranger_C")))