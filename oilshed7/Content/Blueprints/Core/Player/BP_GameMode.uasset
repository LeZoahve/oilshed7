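; BP_GameMode is the game mode, providing the initial random deal of pages into a Book and a Hand.
; DealStartingPages shuffles StartingPlayablePages in place, clears both arrays, then fills the Book and afterwards the Hand up to their configured starting counts.
; It then brackets the Book with two fixed enum pages, one at the front and one at the end.
; BeginPlay, Tick and the construction script are empty.
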(event EventBeginPlay)

(event EventTick
  (params (DeltaSeconds :type Float%20%28single-precision%29)))

(fn ConstructionScript)

(fn DealStartingPages
  (params (Book :type Array%20of%20E_Page%20Enums :default "NewEnumerator0") (Hand :type Array%20of%20E_Page%20Enums :default "NewEnumerator0"))
  (Utilities|FlowControl|Sequence
    (:then_0
      (Utilities|Array|Shuffle (Variables|Default|GetStartingPlayablePages))
      (Utilities|Array|Clear Book)
      (Utilities|Array|Clear Hand))
    (:then_1
      (for _array_element (Variables|Default|GetStartingPlayablePages)
        (if (< (Utilities|Array|Length Book) (Variables|Default|GetStartingPagesInBookCount))
          (Utilities|Array|Add Book _array_element)
          (elif (< (Utilities|Array|Length Hand) (Variables|Default|GetStartingPagesInHandCount))
            (Utilities|Array|Add Hand _array_element)))))
    (:then_2
      (Utilities|Array|Insert Book "NewEnumerator0")
      (Utilities|Array|Add Book "NewEnumerator1"))))