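; BP_PageEffect_BloodPact is a card-game page effect for a spell that hurts its caster as well as the opponent.
; Its CastSpell override calls the parent, then harms the owner by HarmValue and damages the opponent by DamageValue, both flagged as modifiable.
; The event graph holds only disabled default events, so all of the effect's logic lives in that override.
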(event EventBeginPlay
  (|CallParentFunction) ; This node is disabled and will not be called.\nDrag off pins to build functionality.
)

(event Collision|EventActorBeginOverlap
  (params (OtherActor :type Actor%20Object%20Reference))
  (|CallParentFunction OtherActor) ; This node is disabled and will not be called.\nDrag off pins to build functionality.
)

(event EventTick
  (params (DeltaSeconds :type Float%20%28single-precision%29))
  (|CallParentFunction DeltaSeconds) ; This node is disabled and will not be called.\nDrag off pins to build functionality.
)

(fn ConstructionScript
  (|CallParentFunction))

(fn CastSpell
  (params (Modifier :type S%20Modifier%20Structure))
  (|CallParentFunction Modifier)
  (Utilities|FlowControl|Sequence
    (:then_0
      (CallFunction|HarmOwner (Variables|Default|GetHarmValue) true))
    (:then_1
      (CallFunction|DamageOpponent (Variables|Default|GetDamageValue) true))))