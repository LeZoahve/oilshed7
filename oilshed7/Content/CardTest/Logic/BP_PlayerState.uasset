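; BP_PlayerState holds a player's state for the card game: HP, a Book and a Hand.
; A Start event calls Init, which resets HP to its initial value and constructs fresh BP_Book and BP_Hand objects.
; Independently, BeginPlay spawns a BP_PageEffect_BloodPact actor at its own transform and immediately casts its spell, without waiting for Init.
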(event Custom|Start
  (CallFunction|Init))

(event EventBeginPlay
  (bind _returnvalue (Game|SpawnActorfromClass "/Game/CardTest/Logic/Effects/BP_PageEffect_BloodPact.BP_PageEffect_BloodPact_C" (Transformation|GetActorTransform) "Undefined" "MultiplyWithRoot" 0 "NewEnumerator0" 0))
  (Default|CastSpell _returnvalue))

(event EventTick
  (params (DeltaSeconds :type Float%20%28single-precision%29)))

(fn ConstructionScript)

(fn Init
  (Utilities|FlowControl|Sequence
    (:then_0
      (Variables|Default|SetHP (Variables|Default|GetInitialHP)))
    (:then_1
      (bind _returnvalue (Game|ConstructObjectfromClass "/Game/CardTest/Logic/BP_Book.BP_Book_C"))
      (Variables|Default|SetBook _returnvalue)
      (bind _returnvalue_2 (Game|ConstructObjectfromClass "/Game/CardTest/Logic/BP_Hand.BP_Hand_C"))
      (Variables|Default|SetHand _returnvalue_2))))