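; Level loading actor that keeps one streaming sublevel active at a time, loading its InitialLevel on BeginPlay.
; LoadLevel ignores a request for the already loaded level; otherwise it unloads and hides the current streaming level, then records the new name and sets it to load and become visible.
; An invalid level name prints an on-screen error.
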(event EventBeginPlay
  (CallFunction|LoadLevel (Variables|Default|GetInitialLevel)))

(event Collision|EventActorBeginOverlap
  (params (OtherActor :type Actor%20Object%20Reference)))

(event EventTick
  (params (DeltaSeconds :type Float%20%28single-precision%29)))

(fn ConstructionScript)

(fn LoadLevel
  (params (Level :type String))
  (if (Utilities|Enum|NotEqual(Enum) Level (Variables|Default|GetLoadedLevel))
    (Utilities|FlowControl|Sequence
      (:then_0
        (Utilities|IsValid (Class|GameplayStatics|GetStreamingLevel (Utilities|String|StringToName (Variables|Default|GetLoadedLevel)))
          (:Is%20Valid
            (Variables|/Script/Engine.LevelStreaming|SetbShouldBeLoaded (Class|GameplayStatics|GetStreamingLevel (Utilities|String|StringToName (Variables|Default|GetLoadedLevel))) false)
            (Variables|/Script/Engine.LevelStreaming|SetbShouldBeVisible (Class|GameplayStatics|GetStreamingLevel (Utilities|String|StringToName (Variables|Default|GetLoadedLevel))) false))))
      (:then_1
        (bind _output_get (Variables|Default|SetLoadedLevel Level))
        (Utilities|IsValid (Class|GameplayStatics|GetStreamingLevel (Utilities|String|StringToName _output_get))
          (:Is%20Valid
            (Variables|/Script/Engine.LevelStreaming|SetbShouldBeLoaded (Class|GameplayStatics|GetStreamingLevel (Utilities|String|StringToName _output_get)) true)
            (Variables|/Script/Engine.LevelStreaming|SetbShouldBeVisible (Class|GameplayStatics|GetStreamingLevel (Utilities|String|StringToName _output_get)) true))
          (:Is%20Not%20Valid
            (Development|PrintString (Utilities|String|Append "Error - LoadLevel - Invalid : " (Variables|Default|GetLoadedLevel)) true true "(R=1.000000,G=0.034090,B=0.000000,A=1.000000)" 5.0)))))))