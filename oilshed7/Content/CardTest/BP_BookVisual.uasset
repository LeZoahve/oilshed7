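; Book visual actor that spawns a stack of BP_PageVisual pages from BookPages on BeginPlay and animates turning them forward and back.
; Pages and ReadPages hold the unread and read stacks, with page thickness setting offsets.
; Timelines lerp each page between stacks with a half-turn and added height, while DoOnce gates block overlapping same-direction turns.
; Turning back can loop at variable speed to reset the book, automatically after the last page.
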(event Custom|TurnPage
  (params (AllowTurnLastPageAndReset :type Boolean))
  (bind _returnvalue (Transformation|GetActorTransform))
  (bind _currentpage (Variables|Default|GetCurrentPage))
  (bind _returnvalue_2 (Transformation|GetActorTransform _currentpage))
  (bind (_location _rotation _scale) (Math|Transform|BreakTransform _returnvalue))
  (Utilities|FlowControl|DoOnce false :!label _label
    (:Completed
      (if (or AllowTurnLastPageAndReset (> (Utilities|Array|Length (Variables|Default|GetPages)) 1))
        (Utilities|IsValid _currentpage
          (:Is%20Valid
            (Variables|Default|SetReadFromTransform _returnvalue_2)
            (Variables|Default|SetReadToTransform (Math|Transform|MakeTransform (+ _location (Math|Transform|TransformDirection _returnvalue (+ (Variables|Default|GetReadPagesBaseRelativePosition) (* (Utilities|Array|Length (Variables|Default|GetReadPages)) (Variables|Default|GetPageThickness))))) (Math|Transform|TransformRotation _returnvalue_2 "0.000000,179.990000,0.000000") _scale))
            (bind (_direction _animaddedheight _animtransform) (Timeline|Timeline_Turn PlayFromStart)
              (:Update
                (Transformation|SetActorTransform (Variables|Default|GetCurrentPage) (Math|Transform|MakeTransform (+ (Math|Transform|TransformDirection (Transformation|GetActorTransform) (* _animaddedheight "0.000000,30.000000,0.000000")) (.location (Math|Transform|Lerp(Transform) (Variables|Default|GetReadFromTransform) (Variables|Default|GetReadToTransform) _animtransform))) (.rotation (Math|Transform|Lerp(Transform) (Variables|Default|GetReadFromTransform) (Variables|Default|GetReadToTransform) _animtransform)) (.scale (Math|Transform|Lerp(Transform) (Variables|Default|GetReadFromTransform) (Variables|Default|GetReadToTransform) _animtransform)))))
              (:Finished
                (Utilities|Array|Add (Variables|Default|GetReadPages) (Variables|Default|GetCurrentPage))
                (Utilities|Array|RemoveIndex (Variables|Default|GetPages))
                (CallFunction|UpdateCurrentPages)
                (if (Utilities|Array|IsEmpty (Variables|Default|GetPages))
                  (CallFunction|TurnBackPage true 2.0)
                  (goto _label Reset)
                  (else
                    (goto _label Reset)))))))))))

(event Custom|ResetBook
  ;[1 1 1] Editor Events
  (CallFunction|TurnBackPage true 3.0))

(event Custom|TurnBackPage
  (params (LoopUntilReset :type Boolean) (AnimSpeedRatio :type Float%20%28double-precision%29))
  (bind _returnvalue (Transformation|GetActorTransform))
  (bind _currentreadpage (Variables|Default|GetCurrentReadPage))
  (bind _readpages (Variables|Default|GetReadPages))
  (bind _returnvalue_2 (Transformation|GetActorTransform _currentreadpage))
  (bind (_location _rotation _scale) (Math|Transform|BreakTransform _returnvalue))
  (Components|Timeline|SetPlayRate (Variables|Default|GetTimeline_TurnBack) AnimSpeedRatio)
  (Utilities|FlowControl|DoOnce false :!label _label
    (:Completed
      (Utilities|IsValid _currentreadpage :!label _label_2
        (:Is%20Valid
          (Variables|Default|SetReadFromTransform _returnvalue_2)
          (Variables|Default|SetReadToTransform (Math|Transform|MakeTransform (+ _location (Math|Transform|TransformDirection _returnvalue (* (Utilities|Array|Length (Variables|Default|GetPages)) (Variables|Default|GetPageThickness)))) (Math|Transform|TransformRotation _returnvalue_2 "0.000000,-179.990000,0.000000") _scale))
          (bind (_direction _animaddedheight _animtransform) (Timeline|Timeline_TurnBack PlayFromStart)
            (:Update
              (Transformation|SetActorTransform (Variables|Default|GetCurrentReadPage) (Math|Transform|MakeTransform (+ (Math|Transform|TransformDirection (Transformation|GetActorTransform) (* _animaddedheight "0.000000,30.000000,0.000000")) (.location (Math|Transform|Lerp(Transform) (Variables|Default|GetReadFromTransform) (Variables|Default|GetReadToTransform) _animtransform))) (.rotation (Math|Transform|Lerp(Transform) (Variables|Default|GetReadFromTransform) (Variables|Default|GetReadToTransform) _animtransform)) (.scale (Math|Transform|Lerp(Transform) (Variables|Default|GetReadFromTransform) (Variables|Default|GetReadToTransform) _animtransform)))))
            (:Finished
              (Utilities|Array|Insert (Variables|Default|GetPages) (Variables|Default|GetCurrentReadPage))
              (Utilities|Array|RemoveIndex _readpages (Utilities|Array|LastIndex _readpages))
              (CallFunction|UpdateCurrentPages)
              (if (and (Utilities|Array|IsNotEmpty (Variables|Default|GetReadPages)) LoopUntilReset)
                (goto _label_2)
                (else
                  (goto _label Reset))))))))))

(event Custom|TurnOnePage
  ;[1 1 1] Editor Events
  (CallFunction|TurnPage true))

(event Custom|TurnBackOnePage
  ;[1 1 1] Editor Events
  (CallFunction|TurnBackPage false 1.0))

(event EventBeginPlay
  (CallFunction|SpawnPages))

(fn ConstructionScript)

(fn SpawnPages
  (bind _returnvalue (Transformation|GetActorTransform))
  (Variables|Default|SetCurrentPage 0)
  (Utilities|Array|Clear (Variables|Default|GetPages))
  (Utilities|Array|Clear (Variables|Default|GetReadPages))
  (if (Utilities|Array|IsEmpty (Variables|Default|GetBookPages))
    (return)
    (else
      (bind (_arrayindex _arrayelement) (Utilities|Array|ReverseforEachLoop (Variables|Default|GetBookPages))
        (:LoopBody
          (LocalVariables|Setindex _arrayindex)
          (bind _returnvalue_2 (Game|SpawnActorfromClass "/Game/CardTest/BP_PageVisual.BP_PageVisual_C" (Math|Transform|MakeTransform (+ (.location _returnvalue) (Math|Transform|TransformDirection (Transformation|GetActorTransform) (* (Variables|Default|GetPageThickness) (- (Utilities|Array|Length (Variables|Default|GetBookPages)) (+ (LocalVariables|Getindex) 1))))) (.rotation _returnvalue) (.scale _returnvalue)) "Undefined" "MultiplyWithRoot" 0 _arrayelement 0))
          (Utilities|Array|Insert (Variables|Default|GetPages) _returnvalue_2))
        (:Completed
          (CallFunction|UpdateCurrentPages)
          (return))))))

(fn UpdateCurrentPages
  (bind _pages (Variables|Default|GetPages))
  (bind _readpages (Variables|Default|GetReadPages))
  (Utilities|FlowControl|Sequence
    (:then_0
      (if (Utilities|Array|IsEmpty _pages)
        (Variables|Default|SetCurrentPage 0)
        (else
          (Variables|Default|SetCurrentPage (Utilities|Array|Get(acopy) _pages)))))
    (:then_1
      (if (Utilities|Array|IsEmpty _readpages)
        (Variables|Default|SetCurrentReadPage 0)
        (else
          (Variables|Default|SetCurrentReadPage (Utilities|Array|Get(acopy) _readpages (Utilities|Array|LastIndex (Variables|Default|GetReadPages)))))))))