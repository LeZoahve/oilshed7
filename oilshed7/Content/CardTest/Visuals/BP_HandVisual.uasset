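; BP_HandVisual is an actor that displays a hand of page cards (BP_PageVisual), with events to spawn, select, remove or bind pages to a book.
; SpacialDistribute fans pages into an arc, storing target positions and rotations in maps keyed by page.
; Tick interpolates pages toward those targets, dropping entries once reached.
; Selection offsets the chosen page's target and applies the opposite offset to the previous one.
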(event Custom|SelectPage
  (params (PageIndex :type Integer))
  (bind _found (CallFunction|SetSelectedPagefromIndex PageIndex))
  (Variables|Default|SetSelectedIndex (Math|Integer|SelectInt PageIndex -1 _found)))

(event Custom|SelectPreviousPage
  ;[1 1 1] Editor Events
  (bind _result (Math|Integer|DecrementInt (Variables|Default|GetSelectedIndex))
    (:%20%20
      (CallFunction|SelectPage _result))))

(event Custom|SelectNextPage
  ;[1 1 1] Editor Events
  (bind _result (Math|Integer|IncrementInt (Variables|Default|GetSelectedIndex))
    (:%20%20
      (CallFunction|SelectPage _result))))

(event Custom|BindSelectedPageToBook
  (params (Book :type BP%20Book%20Visual%20Object%20Reference))
  (bind _selectedpage (Variables|Default|GetSelectedPage))
  (Utilities|IsValid _selectedpage
    (:Is%20Valid
      (Default|BindPage Book _selectedpage)
      (CallFunction|RemovePage _selectedpage false false))))

(event Custom|AddRandomPage
  ;[1 1 1] Editor Events
  (CallFunction|SpawnPage (Utilities|Enum|ByteToEnumE_Page (Math|Conversions|ToByte(Integer) (Math|Random|RandomInteger (|GetNumEnumEntries))))))

(event Custom|RemoveSelectedPage
  ;[1 1 1] Editor Events
  (CallFunction|RemovePage (Variables|Default|GetSelectedPage) true true))

(event Custom|Spawn
  ;[1 1 1] Editor Events
  (CallFunction|SpawnStartingPages))

(event EventBeginPlay)

(event EventTick
  (params (DeltaSeconds :type Float%20%28single-precision%29))
  (Variables|Default|SetDelta%20Seconds DeltaSeconds)
  (CallFunction|UpdatePagesDistribution))

(fn ConstructionScript)

(fn SpawnStartingPages
  (Variables|Default|SetSelectedPage 0)
  (Utilities|Array|Clear (Variables|Default|GetPages))
  (for _array_element (Variables|Params|GetHandStartingPages)
    (bind _returnvalue (Game|SpawnActorfromClass "/Game/CardTest/Visuals/BP_PageVisual.BP_PageVisual_C" (Transformation|GetActorTransform) "Undefined" "MultiplyWithRoot" 0 _array_element 0))
    (Utilities|Array|Add (Variables|Default|GetPages) _returnvalue)
    (Transformation|AttachActorToActor _returnvalue self "None" "KeepWorld" "KeepWorld" "KeepWorld" false))
  (CallFunction|SpacialDistribute)
  (return))

(fn SpawnPage
  (params (Page :type E_Page%20Enum :default "NewEnumerator0"))
  (bind _returnvalue (Game|SpawnActorfromClass "/Game/CardTest/Visuals/BP_PageVisual.BP_PageVisual_C" (Transformation|GetActorTransform) "Undefined" "MultiplyWithRoot" 0 Page 0))
  (Utilities|Array|Add (Variables|Default|GetPages) _returnvalue)
  (Transformation|AttachActorToActor _returnvalue self "None" "KeepWorld" "KeepWorld" "KeepWorld" false)
  (CallFunction|SpacialDistribute))

(fn RemovePage
  (params (Page :type BP%20Page%20Visual%20Object%20Reference) (AndDetach :type Boolean) (AndDestroy :type Boolean))
  (Utilities|Array|RemoveItem (Variables|Default|GetPages) Page)
  (Utilities|Map|Remove (Variables|Default|GetDesiredPositionsMap) Page)
  (Utilities|Map|Remove (Variables|Default|GetDesiredRotationsMap) Page)
  (if (== (Variables|Default|GetSelectedPage) Page)
    (Variables|Default|SetSelectedPage 0)
    (Variables|Default|SetSelectedIndex -1)
    (if AndDetach
      (Transformation|DetachFromActor Page "KeepRelative" "KeepRelative" "KeepRelative")))
  (if AndDestroy
    (Actor|DestroyActor Page))
  (CallFunction|SpacialDistribute))

(fn AddPage
  (params (Page :type BP%20Page%20Visual%20Object%20Reference%20%28by%20ref%29))
  (Utilities|Array|Add (Variables|Default|GetPages) Page)
  (CallFunction|SpacialDistribute))

(fn SpacialDistribute
  (bind _distributionspacing (Variables|Params|GetDistributionSpacing))
  (Utilities|Map|Clear (Variables|Default|GetDesiredPositionsMap))
  (Utilities|Map|Clear (Variables|Default|GetDesiredRotationsMap))
  (if (Utilities|Array|IsEmpty (Variables|Default|GetPages))
    (return)
    (else
      (LocalVariables|SetPageCount (Utilities|Array|Length (Variables|Default|GetPages)))
      (for (_array_element _array_index) (Variables|Default|GetPages)
        (LocalVariables|SetCurrentPage _array_element)
        (LocalVariables|SetPageIndex _array_index)
        (LocalVariables|SetCurrentSpatialModifier (/ (- (* (LocalVariables|GetPageIndex) 2) (- (LocalVariables|GetPageCount) 1)) 2.0))
        (Utilities|Map|Add (Variables|Default|GetDesiredPositionsMap) (LocalVariables|GetCurrentPage) (+ (Transformation|GetActorLocation) (Math|Transform|TransformDirection (Transformation|GetActorTransform) (Math|Vector|MakeVector (* (LocalVariables|GetCurrentSpatialModifier) (.x _distributionspacing)) (* (.y _distributionspacing) (LocalVariables|GetPageIndex)) (* (Math|Float|Absolute(Float) (Math|Trig|Tan(Degrees) (* (LocalVariables|GetCurrentSpatialModifier) (Variables|Params|GetDistributionAngle)))) (* (.x (Variables|Params|GetDistributionSpacing)) -2.0))))))
        (Utilities|Map|Add (Variables|Default|GetDesiredRotationsMap) (LocalVariables|GetCurrentPage) (Math|Transform|TransformRotation (Transformation|GetActorTransform) (Math|Rotator|MakeRotator 0.0 (* (LocalVariables|GetCurrentSpatialModifier) (Variables|Params|GetDistributionAngle)) 0.0))))
      (return))))

(fn UpdatePagesDistribution
  (Utilities|FlowControl|Sequence
    (:then_0
      (bind _keys (Utilities|Map|Keys (Variables|Default|GetDesiredPositionsMap)))
      (for _array_element _keys
        (LocalVariables|SetCurrentPage _array_element)
        (LocalVariables|SetCurrentPosition (Transformation|GetActorLocation (LocalVariables|GetCurrentPage)))
        (if (.ReturnValue (Utilities|Map|Find (Variables|Default|GetDesiredPositionsMap) (LocalVariables|GetCurrentPage)))
          (LocalVariables|SetCurrentDesiredPosition (.Value (Utilities|Map|Find (Variables|Default|GetDesiredPositionsMap) (LocalVariables|GetCurrentPage))))
          (if (Utilities|Operators|EqualEqual (LocalVariables|GetCurrentPosition) (LocalVariables|GetCurrentDesiredPosition) 0.01)
            (Utilities|Map|Remove (Variables|Default|GetDesiredPositionsMap) (LocalVariables|GetCurrentPage))
            (else
              (Transformation|SetActorLocation (LocalVariables|GetCurrentPage) (Math|Interpolation|VInterpTo (LocalVariables|GetCurrentPosition) (LocalVariables|GetCurrentDesiredPosition) (Variables|Default|GetDelta%20Seconds) (Variables|Params|GetDistributionSpeed)) false false))))))
    (:then_1
      (bind _keys_2 (Utilities|Map|Keys (Variables|Default|GetDesiredRotationsMap)))
      (for _array_element_2 _keys_2
        (LocalVariables|SetCurrentPage _array_element_2)
        (LocalVariables|SetCurrentRotation (Transformation|GetActorRotation (LocalVariables|GetCurrentPage)))
        (if (.ReturnValue (Utilities|Map|Find (Variables|Default|GetDesiredRotationsMap) (LocalVariables|GetCurrentPage)))
          (LocalVariables|SetCurrentDesiredRotation (.Value (Utilities|Map|Find (Variables|Default|GetDesiredRotationsMap) (LocalVariables|GetCurrentPage))))
          (if (Utilities|Operators|EqualEqual (LocalVariables|GetCurrentRotation) (LocalVariables|GetCurrentDesiredRotation) 0.01)
            (Utilities|Map|Remove (Variables|Default|GetDesiredRotationsMap) (LocalVariables|GetCurrentPage))
            (else
              (Transformation|SetActorRotation (LocalVariables|GetCurrentPage) (Math|Interpolation|RInterpTo (LocalVariables|GetCurrentRotation) (LocalVariables|GetCurrentDesiredRotation) (Variables|Default|GetDelta%20Seconds) (Variables|Params|GetDistributionSpeed))))))))))

(fn SetSelectedPagefromIndex
  (params (PageIndex :type Integer))
  (if (<= PageIndex (Utilities|Array|Length (Variables|Default|GetPages)))
    (CallFunction|SelectPageandShowPage (Utilities|Array|Get(acopy) (Variables|Default|GetPages) PageIndex))
    (return true)
    (else
      (return false))))

(fn SelectPageandShowPage
  (params (NewSelectedPage :type BP%20Page%20Visual%20Object%20Reference))
  (Utilities|FlowControl|Sequence
    (:then_0
      (Utilities|IsValid (Variables|Default|GetSelectedPage)
        (:Is%20Valid
          (LocalVariables|SetDisplacement (CallFunction|ComputeSelectionDisplacement false)))))
    (:then_1
      (bind _output_get (Variables|Default|SetSelectedPage NewSelectedPage))
      (Utilities|IsValid _output_get
        (:Is%20Valid
          (LocalVariables|SetDisplacement (CallFunction|ComputeSelectionDisplacement true))))))
  (LocalVariables|SetCurrentSelectedPageTransform (Transformation|GetActorTransform (Variables|Default|GetSelectedPage)))
  (if (.ReturnValue (Utilities|Map|Find (Variables|Default|GetDesiredPositionsMap) (Variables|Default|GetSelectedPage)))
    (LocalVariables|SetDesiredPosition (+ (Math|Transform|TransformDirection (LocalVariables|GetCurrentSelectedPageTransform) (LocalVariables|GetDisplacement)) (.Value (Utilities|Map|Find (Variables|Default|GetDesiredPositionsMap) (Variables|Default|GetSelectedPage)))))
    (else
      (LocalVariables|SetDesiredPosition (+ (Math|Transform|TransformDirection (LocalVariables|GetCurrentSelectedPageTransform) (LocalVariables|GetDisplacement)) (.location (LocalVariables|GetCurrentSelectedPageTransform))))))
  (Utilities|Map|Add (Variables|Default|GetDesiredPositionsMap) (Variables|Default|GetSelectedPage) (LocalVariables|GetDesiredPosition)))

(fn ComputeSelectionDisplacement
  (params (Selecting :type Boolean))
  (bind _selectionspacing (Variables|Params|GetSelectionSpacing))
  (bind _returnvalue (select Selecting 1.0 -1.0))
  (return (Math|Vector|MakeVector 0.0 (* (+ (* (.y (Variables|Params|GetDistributionSpacing)) (Utilities|Array|Length (Variables|Default|GetPages))) (.y _selectionspacing)) _returnvalue) (* (.z _selectionspacing) _returnvalue))))