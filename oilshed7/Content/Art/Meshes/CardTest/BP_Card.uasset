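; BP_Card is a card actor whose front texture, back texture and color are applied to its static mesh at construction.
; The construction script creates separate dynamic instances of MI_CardInstance for the front and back material slots, each fed its own texture.
; It then pushes the Color value as a vector parameter across the mesh's materials.
; The event graph holds only disabled placeholder events, so there is no runtime logic.
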(event EventBeginPlay)

(event Collision|EventActorBeginOverlap
  (params (OtherActor :type Actor%20Object%20Reference)))

(event EventTick
  (params (DeltaSeconds :type Float%20%28single-precision%29)))

(fn ConstructionScript
  (Utilities|FlowControl|Sequence
    (:then_0
      (bind _returnvalue (Rendering|Material|CreateDynamicMaterialInstance "/Game/Art/Meshes/CardTest/MI_CardInstance.MI_CardInstance" "None" "None" :!class /Script/Engine.KismetMaterialLibrary))
      (bind _output_get (LocalVariables|SetCardFront _returnvalue))
      (Rendering|Material|SetTextureParameterValue _output_get "Texture" (Variables|Default|GetFrontTexture))
      (Rendering|Material|SetMaterial (Variables|Default|GetStaticMesh) 0 (LocalVariables|GetCardFront)))
    (:then_1
      (bind _returnvalue_2 (Rendering|Material|CreateDynamicMaterialInstance "/Game/Art/Meshes/CardTest/MI_CardInstance.MI_CardInstance" "None" "None" :!class /Script/Engine.KismetMaterialLibrary))
      (bind _output_get_2 (LocalVariables|SetCardBack _returnvalue_2))
      (Rendering|Material|SetTextureParameterValue _output_get_2 "Texture" (Variables|Default|GetBackTexture))
      (Rendering|Material|SetMaterial (Variables|Default|GetStaticMesh) 2 (LocalVariables|GetCardBack)))
    (:then_2
      (Rendering|Material|SetVectorParameterValueonMaterials (Variables|Default|GetStaticMesh) "Color" (Math|Conversions|ToVector(LinearColor) (Variables|Default|GetColor))))))