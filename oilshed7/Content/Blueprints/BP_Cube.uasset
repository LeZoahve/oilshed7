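; BP_Cube is a cube that displays a countdown on four text components and starts simulating physics when it reaches zero.
; The construction script sets the initial text, and each EDITOR_PassTurn call decrements the count, clamped at zero, refreshes the text and checks for expiry.
; For debugging, DEBUGStartTimer enables a Tick-driven timer that runs the same decrement and check every three seconds.
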(event Custom|EDITOR_PassTurn
  (CallFunction|DecrementCountdown)
  (CallFunction|CheckCountdown))

(event EventBeginPlay)

(event Collision|EventActorBeginOverlap
  (params (OtherActor :type Actor%20Object%20Reference)))

(event EventTick
  (params (DeltaSeconds :type Float%20%28single-precision%29))
  (Debug|DEBUGHandleElapsedTimerTime DeltaSeconds))

(fn ConstructionScript
  (CallFunction|SetCountdownText))

(fn SetCountdownText
  (bind _countdown (Variables|Default|GetCountdown))
  (bind _returnvalue (Utilities|Text|ToText(Integer) _countdown))
  (Rendering|Components|TextRender|SetText (Variables|Default|GetTXT_Right) _returnvalue)
  (Rendering|Components|TextRender|SetText (Variables|Default|GetTXT_Rear) _returnvalue)
  (Rendering|Components|TextRender|SetText (Variables|Default|GetTXT_Left) _returnvalue)
  (Rendering|Components|TextRender|SetText (Variables|Default|GetTXT_Face) _returnvalue))

(fn DecrementCountdown
  (Variables|Default|SetCountdown (Math|Integer|Max(Integer) (- (Variables|Default|GetCountdown) 1)))
  (CallFunction|SetCountdownText))

(fn CheckCountdown
  (if (<= (Variables|Default|GetCountdown) 0)
    (Physics|SetSimulatePhysics (Variables|Default|GetSM_Cube) true)))

(fn DEBUGHandleElapsedTimerTime
  (params (elapsedTime :type Float%20%28double-precision%29))
  (if (Variables|Debug|GetDEBUG_ShouldDecrementOnTimer)
    (bind _output_get (Variables|Debug|SetDEBUG_Timer (+ elapsedTime (Variables|Debug|GetDEBUG_Timer))))
    (if (>= _output_get 3.0)
      (Variables|Debug|SetDEBUG_Timer 0.0)
      (CallFunction|DecrementCountdown)
      (CallFunction|CheckCountdown))))

(fn DEBUGStartTimer
  (Variables|Debug|SetDEBUG_ShouldDecrementOnTimer true))