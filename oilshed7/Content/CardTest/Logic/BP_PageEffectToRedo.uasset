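; Page effect Blueprint for a Grimoires card game that applies a page's turn effects to player states.
; Construction loads the effect list from page data, and TurnPage dispatches each entry to helpers for opponent damage, owner healing or harm, inspiration and manipulations.
; Modifiable effects go through ModifyValue, which applies the stored spell modifier to zero instead of the incoming value.
; CastSpell only stores that modifier.
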(event EventBeginPlay)

(event Collision|EventActorBeginOverlap
  (params (OtherActor :type Actor%20Object%20Reference)))

(event EventTick
  (params (DeltaSeconds :type Float%20%28single-precision%29)))

(fn ConstructionScript
  (bind _pagedata (CallFunction|GetPageData (Variables|Default|GetPage)))
  (Variables|Default|SetTurn%20Page%20Effect (.TurnPageEffect (Utilities|Struct|BreakS_PageData _pagedata))))

(fn CastSpell
  (params (Modifier :type S%20Modifier%20Structure))
  (Variables|Default|SetModifier Modifier))

(fn ModifyValue
  (params (Value :type Integer))
  (LocalVariables|SetModifier (.value (Variables|Default|GetModifier)))
  (switch Utilities|FlowControl|Switch|SwitchonE_ModifierType (.modifiertype (Variables|Default|GetModifier))
    (:NewEnumerator0
      (LocalVariables|SetFinalValue 0))
    (:NewEnumerator1
      (LocalVariables|SetFinalValue (+ 0 (LocalVariables|GetModifier))))
    (:NewEnumerator2
      (LocalVariables|SetFinalValue (Math|Integer|Max(Integer) (- 0 (LocalVariables|GetModifier)))))
    (:NewEnumerator3
      (LocalVariables|SetFinalValue (* 0 (LocalVariables|GetModifier)))))
  (return (LocalVariables|GetFinalValue)))

(fn HealOwner
  (params (Value :type Integer) (Modifiable :type Boolean))
  (bind _playerstate (CallFunction|GetLocalPlayerState))
  (Utilities|IsValid _playerstate
    (:Is%20Valid
      (bind _asgrimoires_player_state (Utilities|Casting|CastToGrimoiresPlayerState _playerstate))
      (Class|GrimoiresPlayerState|GainHP _asgrimoires_player_state (Math|Integer|SelectInt (CallFunction|ModifyValue Value) Value Modifiable)))))

(fn HarmOwner
  (params (Value :type Integer) (Modifiable :type Boolean))
  (bind _playerstate (CallFunction|GetLocalPlayerState))
  (Utilities|IsValid _playerstate
    (:Is%20Valid
      (bind _asgrimoires_player_state (Utilities|Casting|CastToGrimoiresPlayerState _playerstate))
      (Class|GrimoiresPlayerState|LoseHP _asgrimoires_player_state (Math|Integer|SelectInt (CallFunction|ModifyValue Value) Value Modifiable)))))

(fn DamageOpponent
  (params (Value :type Integer) (Modifiable :type Boolean))
  (bind _playerstate (CallFunction|GetOpponentPlayerState))
  (Utilities|IsValid _playerstate
    (:Is%20Valid
      (bind _asgrimoires_player_state (Utilities|Casting|CastToGrimoiresPlayerState _playerstate))
      (Class|GrimoiresPlayerState|LoseHP _asgrimoires_player_state (Math|Integer|SelectInt (CallFunction|ModifyValue Value) Value Modifiable)))))

(fn TurnPage
  (for _array_element (Variables|Default|GetTurn%20Page%20Effect)
    (LocalVariables|SetValue (.Value (Utilities|Struct|BreakS_SpellEffect _array_element)))
    (LocalVariables|SetModifiable (.Modifiable (Utilities|Struct|BreakS_SpellEffect _array_element)))
    (switch Utilities|FlowControl|Switch|SwitchonE_SpellEffectType (.Type (Utilities|Struct|BreakS_SpellEffect _array_element))
      (:NewEnumerator0
        (Effects|DamageOpponent (LocalVariables|GetValue) (LocalVariables|GetModifiable)))
      (:NewEnumerator1
        (Effects|HealOwner (LocalVariables|GetValue) (LocalVariables|GetModifiable)))
      (:NewEnumerator2
        (Effects|HarmOwner (LocalVariables|GetValue) (LocalVariables|GetModifiable)))
      (:NewEnumerator3
        (Effects|UpdateInspiration (LocalVariables|GetValue) (LocalVariables|GetModifiable)))
      (:NewEnumerator4
        (Effects|UpdateManipulations (LocalVariables|GetValue) (LocalVariables|GetModifiable)))
      (:NewEnumerator12
        (Effects|UpdateManipulations (* (LocalVariables|GetValue) -1) (LocalVariables|GetModifiable))))))

(fn UpdateInspiration
  (params (Value :type Integer) (Modifiable :type Boolean))
  (bind _playerstate (CallFunction|GetLocalPlayerState))
  (Utilities|IsValid _playerstate
    (:Is%20Valid
      (bind _asgrimoires_player_state (Utilities|Casting|CastToGrimoiresPlayerState _playerstate))
      (Class|GrimoiresPlayerState|UpdateInspiration _asgrimoires_player_state (Math|Integer|SelectInt (CallFunction|ModifyValue Value) Value Modifiable)))))

(fn UpdateManipulations
  (params (Value :type Integer) (Modifiable :type Boolean))
  (bind _playerstate (CallFunction|GetLocalPlayerState))
  (Utilities|IsValid _playerstate
    (:Is%20Valid
      (bind _asgrimoires_player_state (Utilities|Casting|CastToGrimoiresPlayerState _playerstate))
      (Class|GrimoiresPlayerState|UpdateManipulations _asgrimoires_player_state (Math|Integer|SelectInt (CallFunction|ModifyValue Value) Value Modifiable)))))