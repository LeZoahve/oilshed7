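; Visual actor for a book whose pages can be turned, turned back, peeked, bound in or ripped out to a hand.
; Spawns page actors as an attached stack, tracking unread and read pages in two arrays whose top pages drive each action.
; Timelines lerp pages between computed stack transforms, arcing turns and looping faster turn-backs to reset.
; Gameplay requests enter an event queue that runs one at a time, each finished action starting the next.
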(event Custom|TurnBackOnePage
  ;[1 1 1] Editor Events
  (CallFunction|InternalTurnBackPage false 1.0))

(event Custom|Spawn
  ;[1 1 1] Editor Events
  (CallFunction|SpawnStartingPages))

(event Custom|RipReadPage
  (params (HandDestination :type BP%20Hand%20Visual%20Object%20Reference%20%28by%20ref%29))
  (Variables|Stack|SetHandForRip HandDestination)
  (StackHandling|StartorStack "NewEnumerator4"))

(event Custom|TurnOnePage
  ;[1 1 1] Editor Events
  (CallFunction|InternalTurnPage true))

(event Custom|Peek
  ;[1 1 1] Editor Events
  (CallFunction|InternalPeek 45.0 44.0))

(event Custom|BindPage
  (params (NewPage :type BP%20Page%20Visual%20Object%20Reference%20%28by%20ref%29))
  (Utilities|Array|Add (Variables|Stack|GetPagesToBind) NewPage)
  (StackHandling|StartorStack "NewEnumerator3"))

(event Custom|RipCurrentPage
  (params (HandDestination :type BP%20Hand%20Visual%20Object%20Reference%20%28by%20ref%29))
  (Variables|Stack|SetHandForRip HandDestination)
  (StackHandling|StartorStack "NewEnumerator5"))

(event Custom|TurnPage
  (StackHandling|StartorStack "NewEnumerator0"))

(event Custom|TurnBackPage
  (StackHandling|StartorStack "NewEnumerator2"))

(event Custom|Reset
  (StackHandling|StartorStack "NewEnumerator1"))

(event EventBeginPlay)

(event Custom|Internal_TurnPage
  (params (AllowTurnLastPage :type Boolean))
  (bind _currentpage (Variables|Default|GetCurrentPage))
  (Utilities|FlowControl|DoOnce false :!label _label
    (:Completed
      (if (or AllowTurnLastPage (> (Utilities|Array|Length (Variables|Default|GetPages)) 1))
        (Utilities|IsValid _currentpage
          (:Is%20Valid
            (Variables|Default|SetFromTransform (Transformation|GetActorTransform _currentpage))
            (Variables|Default|SetToTransform (CallFunction|ComputeNextReadPageTransform))
            (bind (_direction _animaddedheight _animtransform) (Timeline|Timeline_Turn PlayFromStart)
              (:Update
                (Transformation|SetActorTransform (Variables|Default|GetCurrentPage) (Math|Transform|MakeTransform (+ (Math|Transform|TransformDirection (Transformation|GetActorTransform) (* _animaddedheight "0.000000,30.000000,0.000000")) (.location (Math|Transform|Lerp(Transform) (Variables|Default|GetFromTransform) (Variables|Default|GetToTransform) _animtransform))) (.rotation (Math|Transform|Lerp(Transform) (Variables|Default|GetFromTransform) (Variables|Default|GetToTransform) _animtransform)) (.scale (Math|Transform|Lerp(Transform) (Variables|Default|GetFromTransform) (Variables|Default|GetToTransform) _animtransform)))))
              (:Finished
                (Utilities|Array|Add (Variables|Default|GetReadPages) (Variables|Default|GetCurrentPage))
                (Utilities|Array|RemoveIndex (Variables|Default|GetPages))
                (CallFunction|UpdateCurrentPages)
                (Utilities|FlowControl|Sequence
                  (:then_0
                    (goto _label Reset))
                  (:then_1
                    (StackHandling|PopandStartNext "NewEnumerator0")))))))))))

(event Custom|Internal_ResetBook
  (CallFunction|InternalTurnBackPage true 3.0))

(event Custom|Internal_TurnBackPage
  (params (LoopUntilReset :type Boolean) (AnimSpeedRatio :type Float%20%28double-precision%29))
  (bind _currentreadpage (Variables|Default|GetCurrentReadPage))
  (bind _readpages (Variables|Default|GetReadPages))
  (Components|Timeline|SetPlayRate (Variables|Default|GetTimeline_TurnBack) AnimSpeedRatio)
  (Utilities|FlowControl|DoOnce false :!label _label
    (:Completed
      (Utilities|IsValid _currentreadpage :!label _label_2
        (:Is%20Valid
          (Variables|Default|SetFromTransform (Transformation|GetActorTransform _currentreadpage))
          (Variables|Default|SetToTransform (CallFunction|ComputeNextCurrentPageTransform))
          (bind (_direction _animaddedheight _animtransform) (Timeline|Timeline_TurnBack PlayFromStart)
            (:Update
              (Transformation|SetActorTransform (Variables|Default|GetCurrentReadPage) (Math|Transform|MakeTransform (+ (Math|Transform|TransformDirection (Transformation|GetActorTransform) (* _animaddedheight "0.000000,30.000000,0.000000")) (.location (Math|Transform|Lerp(Transform) (Variables|Default|GetFromTransform) (Variables|Default|GetToTransform) _animtransform))) (.rotation (Math|Transform|Lerp(Transform) (Variables|Default|GetFromTransform) (Variables|Default|GetToTransform) _animtransform)) (.scale (Math|Transform|Lerp(Transform) (Variables|Default|GetFromTransform) (Variables|Default|GetToTransform) _animtransform)))))
            (:Finished
              (Utilities|Array|Insert (Variables|Default|GetPages) (Variables|Default|GetCurrentReadPage))
              (Utilities|Array|RemoveIndex _readpages (Utilities|Array|LastIndex _readpages))
              (CallFunction|UpdateCurrentPages)
              (if (and (Utilities|Array|IsNotEmpty (Variables|Default|GetReadPages)) LoopUntilReset)
                (goto _label_2)
                (else
                  (Utilities|FlowControl|Sequence
                    (:then_0
                      (goto _label Reset))
                    (:then_1
                      (StackHandling|PopandStartNext (select LoopUntilReset "NewEnumerator1" "NewEnumerator2")))))))))))))

(event Custom|Internal_Peek
  (params (angle :type Float%20%28double-precision%29) (shift :type Float%20%28double-precision%29))
  (Variables|Default|SetFromTransform (Transformation|GetActorTransform (Variables|Default|GetCurrentPage)))
  (Variables|Default|SetToTransform (CallFunction|ComputePeekTransform angle shift))
  (bind _transformratio (Timeline|Timeline_Peek PlayFromStart)
    (:Update
      (Transformation|SetActorTransform (Variables|Default|GetCurrentPage) (Math|Transform|Lerp(Transform) (Variables|Default|GetFromTransform) (Variables|Default|GetToTransform) _transformratio)))
    (:Finished
      (StackHandling|PopandStartNext "NewEnumerator6"))))

(event Custom|Internal_BindPage
  (params (NewPage :type BP%20Page%20Visual%20Object%20Reference%20%28by%20ref%29))
  (Utilities|FlowControl|Sequence
    (:then_0
      (Variables|Default|SetFromTransform (Transformation|GetActorTransform NewPage))
      (Variables|Default|SetToTransform (CallFunction|ComputeNextReadPageTransform)))
    (:then_1
      (Utilities|Array|Add (Variables|Default|GetReadPages) NewPage)
      (CallFunction|UpdateCurrentPages)
      (bind _newtrack_addtransform (Timeline|Timeline_Bind PlayFromStart)
        (:Update
          (Transformation|SetActorTransform (Variables|Default|GetCurrentReadPage) (Math|Transform|MakeTransform (.location (Math|Transform|Lerp(Transform) (Variables|Default|GetFromTransform) (Variables|Default|GetToTransform) _newtrack_addtransform)) (.rotation (Math|Transform|Lerp(Transform) (Variables|Default|GetFromTransform) (Variables|Default|GetToTransform) _newtrack_addtransform)) (.scale (Math|Transform|Lerp(Transform) (Variables|Default|GetFromTransform) (Variables|Default|GetToTransform) _newtrack_addtransform)))))
        (:Finished
          (Transformation|AttachActorToActor (Variables|Default|GetCurrentReadPage) self "None" "KeepRelative" "KeepRelative" "KeepRelative" true)
          (StackHandling|PopandStartNext "NewEnumerator3"))))))

(event Custom|Internal_RipPage
  (params (FromReadPages :type Boolean) (HandDestination :type BP%20Hand%20Visual%20Object%20Reference%20%28by%20ref%29))
  (bind _readpages (Variables|Default|GetReadPages))
  (if FromReadPages
    (Transformation|DetachFromActor (Variables|Default|GetCurrentReadPage) "KeepRelative" "KeepRelative" "KeepRelative")
    (Default|AddPage HandDestination (Variables|Default|GetCurrentReadPage))
    (Utilities|Array|RemoveIndex _readpages (Utilities|Array|LastIndex _readpages))
    (CallFunction|UpdateCurrentPages)
    (StackHandling|PopandStartNext "NewEnumerator4")
    (else
      (Transformation|DetachFromActor (Variables|Default|GetCurrentPage) "KeepRelative" "KeepRelative" "KeepRelative")
      (Default|AddPage HandDestination (Variables|Default|GetCurrentPage))
      (Utilities|Array|RemoveIndex (Variables|Default|GetPages))
      (CallFunction|UpdateCurrentPages)
      (StackHandling|PopandStartNext "NewEnumerator5"))))

(fn ConstructionScript)

(fn SpawnStartingPages
  (bind _returnvalue (Transformation|GetActorTransform))
  (Variables|Default|SetCurrentPage 0)
  (Utilities|Array|Clear (Variables|Default|GetPages))
  (Utilities|Array|Clear (Variables|Default|GetReadPages))
  (if (Utilities|Array|IsEmpty (Variables|Default|GetBookStartingPages))
    (return)
    (else
      (bind (_arrayindex _arrayelement) (Utilities|Array|ReverseforEachLoop (Variables|Default|GetBookStartingPages))
        (:LoopBody
          (LocalVariables|Setindex _arrayindex)
          (bind _returnvalue_2 (Game|SpawnActorfromClass "/Game/CardTest/Visuals/BP_PageVisual.BP_PageVisual_C" (Math|Transform|MakeTransform (+ (.location _returnvalue) (Math|Transform|TransformDirection (Transformation|GetActorTransform) (* (Variables|Default|GetPageThickness) (- (Utilities|Array|Length (Variables|Default|GetBookStartingPages)) (+ (LocalVariables|Getindex) 1))))) (.rotation _returnvalue) (.scale _returnvalue)) "Undefined" "MultiplyWithRoot" 0 _arrayelement 0))
          (Utilities|Array|Insert (Variables|Default|GetPages) _returnvalue_2)
          (Transformation|AttachActorToActor _returnvalue_2 self "None" "KeepRelative" "KeepRelative" "KeepRelative" true))
        (:Completed
          (CallFunction|UpdateCurrentPages)
          (return))))))

(fn UpdateCurrentPages
  (bind _pages (Variables|Default|GetPages))
  (bind _readpages (Variables|Default|GetReadPages))
  (Utilities|FlowControl|Sequence
    (:then_0
      (if (Utilities|Array|IsEmpty _pages)
        (Variables|Default|SetCurrentPage 0)
        (else
          (Variables|Default|SetCurrentPage (Utilities|Array|Get(acopy) _pages)))))
    (:then_1
      (if (Utilities|Array|IsEmpty _readpages)
        (Variables|Default|SetCurrentReadPage 0)
        (else
          (Variables|Default|SetCurrentReadPage (Utilities|Array|Get(acopy) _readpages (Utilities|Array|LastIndex (Variables|Default|GetReadPages)))))))))

(fn ComputeNextReadPageTransform
  (bind _returnvalue (Transformation|GetActorTransform))
  (bind _readpages (Variables|Default|GetReadPages))
  (bind (_location _rotation _scale) (Math|Transform|BreakTransform _returnvalue))
  (if (Utilities|Array|IsEmpty (Variables|Default|GetReadPages))
    (return (Math|Transform|MakeTransform (+ _location (Math|Transform|TransformDirection _returnvalue (Variables|Default|GetReadPagesBaseRelativePosition))) (Math|Transform|TransformRotation _returnvalue "0.000000,179.990000,0.000000") _scale))
    (else
      (LocalVariables|SetLastReadPage (Utilities|Array|Get(acopy) _readpages (Utilities|Array|LastIndex _readpages)))
      (return (Math|Transform|MakeTransform (+ (.Location (Math|Transform|BreakTransform (Transformation|GetActorTransform (LocalVariables|GetLastReadPage)))) (Math|Transform|TransformDirection (Transformation|GetActorTransform (LocalVariables|GetLastReadPage)) (* (Variables|Default|GetPageThickness) -1.0))) (.Rotation (Math|Transform|BreakTransform (Transformation|GetActorTransform (LocalVariables|GetLastReadPage)))) (.Scale (Math|Transform|BreakTransform (Transformation|GetActorTransform (LocalVariables|GetLastReadPage)))))))))

(fn ComputeNextCurrentPageTransform
  (bind _currentpage (Variables|Default|GetCurrentPage))
  (bind _returnvalue (Transformation|GetActorTransform _currentpage))
  (bind (_location _rotation _scale) (Math|Transform|BreakTransform _returnvalue))
  (if (Utilities|Array|IsEmpty (Variables|Default|GetPages))
    (return (Transformation|GetActorTransform))
    (else
      (return (Math|Transform|MakeTransform (+ _location (Math|Transform|TransformDirection _returnvalue (Variables|Default|GetPageThickness))) _rotation _scale)))))

(fn StartorStack
  (params (Event :type E_BookVisualEvent%20Enum :default "NewEnumerator0"))
  (LocalVariables|SetCanStart (Utilities|Array|IsEmpty (Variables|Stack|GetBookEventStack)))
  (Utilities|Array|Add (Variables|Stack|GetBookEventStack) Event)
  (if (LocalVariables|GetCanStart)
    (StackHandling|StartNextEvent)))

(fn PopandStartNext
  (params (Event :type E_BookVisualEvent%20Enum :default "NewEnumerator0"))
  (if (Utilities|Array|IsNotEmpty (Variables|Stack|GetBookEventStack))
    (if (Utilities|Enum|Equal(Enum) Event (Utilities|Array|Get(acopy) (Variables|Stack|GetBookEventStack)))
      (Utilities|Array|RemoveIndex (Variables|Stack|GetBookEventStack))
      (if (Utilities|Array|IsNotEmpty (Variables|Stack|GetBookEventStack))
        (StackHandling|StartNextEvent)))))

(fn StartNextEvent
  (switch Utilities|FlowControl|Switch|SwitchonE_BookVisualEvent (Utilities|Array|Get(acopy) (Variables|Stack|GetBookEventStack))
    (:NewEnumerator0
      (CallFunction|InternalTurnPage true))
    (:NewEnumerator2
      (CallFunction|InternalTurnBackPage false 1.0))
    (:NewEnumerator1
      (CallFunction|InternalResetBook))
    (:NewEnumerator3
      (CallFunction|InternalBindPage (Utilities|Array|Get(acopy) (Variables|Stack|GetPagesToBind)))
      (Utilities|Array|RemoveIndex (Variables|Stack|GetPagesToBind)))
    (:NewEnumerator4
      (CallFunction|InternalRipPage true (Variables|Stack|GetHandForRip)))
    (:NewEnumerator5
      (CallFunction|InternalRipPage false (Variables|Stack|GetHandForRip)))
    (:NewEnumerator6
      (CallFunction|InternalPeek 45.0 44.0))))

(fn ComputePeekTransform
  (params (Angle :type Float%20%28double-precision%29) (Shift :type Float%20%28double-precision%29))
  (bind _returnvalue (Math|Trig|Sin(Degrees) Angle))
  (bind _returnvalue_2 (* _returnvalue Shift))
  (return (Math|Transform|MakeTransform (Math|Transform|TransformLocation (Transformation|GetActorTransform (Variables|Default|GetCurrentPage)) (Math|Vector|MakeVector 0.0 _returnvalue_2 (- Shift (/ _returnvalue_2 (Math|Trig|Tan(Degrees) Angle))))) (Math|Transform|TransformRotation (Transformation|GetActorTransform (Variables|Default|GetCurrentPage)) (Math|Rotator|MakeRotator (* Angle -1.0) 0.0 0.0)))))