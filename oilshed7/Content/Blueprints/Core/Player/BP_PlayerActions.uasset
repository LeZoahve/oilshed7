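; BP_PlayerActions handles the player's mouse interaction with tiles on the BP_Grid actor found at BeginPlay.
; Each tick it queries the tile index under the cursor and, when that changes, moves a hover state from the old tile to the new one.
; Left click adds a second tile state to the hovered tile and right click removes it, with input enabled through a temporary test hookup.
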(event EventBeginPlay
  (bind _returnvalue (Actor|GetActorOfClass "/Game/Blueprints/Core/Grid/BP_Grid.BP_Grid_C"))
  (Variables|Default|SetGrid _returnvalue)
  ;[1 1 1] Temp test
  (Input|EnableInput (Game|GetPlayerController 0)))

(event EventTick
  (params (DeltaSeconds :type Float%20%28single-precision%29))
  (CallFunction|UpdateTileUnderCursor))

(event Input|MouseEvents|LeftMouseButton
  (params (Key :type Key%20Structure :default "None"))
  ;[1 1 1] Temp test
  (:Pressed
    (Default|AddStatetoTile (Variables|Default|GetGrid) (Variables|Default|GetHoveredTileIndex) "NewEnumerator2")))

(event Input|MouseEvents|RightMouseButton
  (params (Key :type Key%20Structure :default "None"))
  ;[1 1 1] Temp test
  (:Pressed
    (Default|RemoveStatefromTile (Variables|Default|GetGrid) (Variables|Default|GetHoveredTileIndex) "NewEnumerator2")))

(fn ConstructionScript)

(fn UpdateTileUnderCursor
  (bind _index (Default|GetTileIndexUnderCursor (Variables|Default|GetGrid)))
  (if (!= _index (Variables|Default|GetHoveredTileIndex))
    (Default|RemoveStatefromTile (Variables|Default|GetGrid) (Variables|Default|GetHoveredTileIndex) "NewEnumerator1")
    (Variables|Default|SetHoveredTileIndex _index)
    (Default|AddStatetoTile (Variables|Default|GetGrid) (Variables|Default|GetHoveredTileIndex) "NewEnumerator1")))