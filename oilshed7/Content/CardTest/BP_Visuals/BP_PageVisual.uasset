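; Visual actor for a two-sided page or card that flips when the FlipPage event it binds to fires.
; Construction looks up front and back textures from the Page data, applies each through its own dynamic material instance, and sets the mesh color.
; A timeline drives Flip, which applies delta local yaw against the tracked CurrentRotation to turn 180 degrees, reversing when the page is not at zero.
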(event Custom|FlipPageEvent_Callback
  (if (== (Variables|Default|GetCurrentRotation) 0.0)
    (bind _anglefactor (Timeline|Timeline Play)
      (:Update
        (CallFunction|Flip _anglefactor)))
    (else
      (Timeline|Timeline Reverse))))

(event EventBeginPlay
  (EventDispatchers|BindEventtoFlipPage (EventDispatchers|CreateEvent :!event Custom|FlipPageEvent_Callback)))

(event EventTick
  (params (DeltaSeconds :type Float%20%28single-precision%29)))

(fn ConstructionScript
  (Utilities|FlowControl|Sequence
    (:then_0
      (bind _pagedata (CallFunction|GetPageData (Variables|Default|GetPage)))
      (LocalVariables|SetFrontTexture (.fronttexture _pagedata))
      (LocalVariables|SetBackTexture (.backtexture _pagedata)))
    (:then_1
      (bind _returnvalue (Rendering|Material|CreateDynamicMaterialInstance "/Game/CardTest/Art/MI_CardInstance.MI_CardInstance" "None" "None" :!class /Script/Engine.KismetMaterialLibrary))
      (bind _output_get (LocalVariables|SetFrontMaterialInstance _returnvalue))
      (Rendering|Material|SetTextureParameterValue _output_get "Texture" (LocalVariables|GetFrontTexture))
      (Rendering|Material|SetMaterial (Variables|Default|GetStaticMesh) 0 (LocalVariables|GetFrontMaterialInstance)))
    (:then_2
      (bind _returnvalue_2 (Rendering|Material|CreateDynamicMaterialInstance "/Game/CardTest/Art/MI_CardInstance.MI_CardInstance" "None" "None" :!class /Script/Engine.KismetMaterialLibrary))
      (bind _output_get_2 (LocalVariables|SetBackMaterialInstance _returnvalue_2))
      (Rendering|Material|SetTextureParameterValue _output_get_2 "Texture" (LocalVariables|GetBackTexture))
      (Rendering|Material|SetMaterial (Variables|Default|GetStaticMesh) 2 (LocalVariables|GetBackMaterialInstance)))
    (:then_3
      (Rendering|Material|SetVectorParameterValueonMaterials (Variables|Default|GetStaticMesh) "Color" (Math|Conversions|ToVector(LinearColor) (Variables|Default|GetColor))))))

(fn Flip
  (params (factor :type Float%20%28double-precision%29))
  (bind _returnvalue (* factor 1.8e+02))
  (Transformation|AddActorLocalRotation (Math|Rotator|MakeRotator 0.0 0.0 (- _returnvalue (Variables|Default|GetCurrentRotation))) false false)
  (Variables|Default|SetCurrentRotation _returnvalue))