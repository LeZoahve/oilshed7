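; Visual book actor for the card game that spawns a BP_PageVisual per entry in BookPages as a stacked pile.
; Two arrays, Pages and ReadPages, model unread and read stacks, each new transform offset by page thickness.
; Timelines animate turning pages forward with an arc, back singly or looped to reset, and binding new pages.
; Ripping hands a page to a hand; turning the last page auto-rewinds the book.
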(event Custom|TurnPage
  (params (AllowTurnLastPageAndReset :type Boolean))
  (bind _currentpage (Variables|Default|GetCurrentPage))
  (Utilities|FlowControl|DoOnce false :!label _label
    (:Completed
      (if (or AllowTurnLastPageAndReset (> (Utilities|Array|Length (Variables|Default|GetPages)) 1))
        (Utilities|IsValid _currentpage
          (:Is%20Valid
            (Variables|Default|SetReadFromTransform (Transformation|GetActorTransform _currentpage))
            (Variables|Default|SetReadToTransform (CallFunction|ComputeNextReadPageTransform))
            (bind (_direction _animaddedheight _animtransform) (Timeline|Timeline_Turn PlayFromStart)
              (:Update
                (Transformation|SetActorTransform (Variables|Default|GetCurrentPage) (Math|Transform|MakeTransform (+ (Math|Transform|TransformDirection (Transformation|GetActorTransform) (* _animaddedheight "0.000000,30.000000,0.000000")) (.location (Math|Transform|Lerp(Transform) (Variables|Default|GetReadFromTransform) (Variables|Default|GetReadToTransform) _animtransform))) (.rotation (Math|Transform|Lerp(Transform) (Variables|Default|GetReadFromTransform) (Variables|Default|GetReadToTransform) _animtransform)) (.scale (Math|Transform|Lerp(Transform) (Variables|Default|GetReadFromTransform) (Variables|Default|GetReadToTransform) _animtransform)))))
              (:Finished
                (Utilities|Array|Add (Variables|Default|GetReadPages) (Variables|Default|GetCurrentPage))
                (Utilities|Array|RemoveIndex (Variables|Default|GetPages))
                (CallFunction|UpdateCurrentPages)
                (if (Utilities|Array|IsEmpty (Variables|Default|GetPages))
                  (CallFunction|TurnBackPage true 2.0)
                  (goto _label Reset)
                  (else
                    (goto _label Reset)))))))))))

(event Custom|ResetBook
  ;[1 1 1] Editor Events
  (CallFunction|TurnBackPage true 3.0))

(event Custom|TurnBackPage
  (params (LoopUntilReset :type Boolean) (AnimSpeedRatio :type Float%20%28double-precision%29))
  (bind _currentreadpage (Variables|Default|GetCurrentReadPage))
  (bind _readpages (Variables|Default|GetReadPages))
  (Components|Timeline|SetPlayRate (Variables|Default|GetTimeline_TurnBack) AnimSpeedRatio)
  (Utilities|FlowControl|DoOnce false :!label _label
    (:Completed
      (Utilities|IsValid _currentreadpage :!label _label_2
        (:Is%20Valid
          (Variables|Default|SetReadFromTransform (Transformation|GetActorTransform _currentreadpage))
          (Variables|Default|SetReadToTransform (CallFunction|ComputeNextCurrentPageTransform))
          (bind (_direction _animaddedheight _animtransform) (Timeline|Timeline_TurnBack PlayFromStart)
            (:Update
              (Transformation|SetActorTransform (Variables|Default|GetCurrentReadPage) (Math|Transform|MakeTransform (+ (Math|Transform|TransformDirection (Transformation|GetActorTransform) (* _animaddedheight "0.000000,30.000000,0.000000")) (.location (Math|Transform|Lerp(Transform) (Variables|Default|GetReadFromTransform) (Variables|Default|GetReadToTransform) _animtransform))) (.rotation (Math|Transform|Lerp(Transform) (Variables|Default|GetReadFromTransform) (Variables|Default|GetReadToTransform) _animtransform)) (.scale (Math|Transform|Lerp(Transform) (Variables|Default|GetReadFromTransform) (Variables|Default|GetReadToTransform) _animtransform)))))
            (:Finished
              (Utilities|Array|Insert (Variables|Default|GetPages) (Variables|Default|GetCurrentReadPage))
              (Utilities|Array|RemoveIndex _readpages (Utilities|Array|LastIndex _readpages))
              (CallFunction|UpdateCurrentPages)
              (if (and (Utilities|Array|IsNotEmpty (Variables|Default|GetReadPages)) LoopUntilReset)
                (goto _label_2)
                (else
                  (goto _label Reset))))))))))

(event Custom|TurnOnePage
  ;[1 1 1] Editor Events
  (CallFunction|TurnPage true))

(event Custom|TurnBackOnePage
  ;[1 1 1] Editor Events
  (CallFunction|TurnBackPage false 1.0))

(event Custom|BindPage
  (params (NewPage :type BP%20Page%20Visual%20Object%20Reference%20%28by%20ref%29))
  (bind _readpages (Variables|Default|GetReadPages))
  (Utilities|FlowControl|Sequence
    (:then_0
      (Variables|Default|SetReadFromTransform (Transformation|GetActorTransform NewPage))
      (Variables|Default|SetReadToTransform (CallFunction|ComputeNextReadPageTransform)))
    (:then_1
      (Utilities|Array|Add (Variables|Default|GetReadPages) NewPage)
      (CallFunction|UpdateCurrentPages)
      (bind _newtrack_addtransform (Timeline|Timeline_Add PlayFromStart)
        (:Update
          (Transformation|SetActorTransform (Utilities|Array|Get(acopy) _readpages (Utilities|Array|LastIndex _readpages)) (Math|Transform|MakeTransform (.location (Math|Transform|Lerp(Transform) (Variables|Default|GetReadFromTransform) (Variables|Default|GetReadToTransform) _newtrack_addtransform)) (.rotation (Math|Transform|Lerp(Transform) (Variables|Default|GetReadFromTransform) (Variables|Default|GetReadToTransform) _newtrack_addtransform)) (.scale (Math|Transform|Lerp(Transform) (Variables|Default|GetReadFromTransform) (Variables|Default|GetReadToTransform) _newtrack_addtransform)))))))))

(event Custom|RipPage
  (params (FromReadPages :type Boolean) (HandDestination :type BP%20Hand%20Visual%20Object%20Reference%20%28by%20ref%29))
  (bind _readpages (Variables|Default|GetReadPages))
  (bind _readpages_2 (Variables|Default|GetReadPages))
  (if FromReadPages
    (Default|AddPage HandDestination (Utilities|Array|Get(acopy) _readpages_2 (Utilities|Array|LastIndex _readpages_2)))
    (Utilities|Array|RemoveIndex _readpages (Utilities|Array|LastIndex _readpages))
    (else
      (Default|AddPage HandDestination (Utilities|Array|Get(acopy) (Variables|Default|GetPages)))
      (Utilities|Array|RemoveIndex (Variables|Default|GetPages))))
  (CallFunction|UpdateCurrentPages))

(event EventBeginPlay
  (CallFunction|SpawnPages))

(fn ConstructionScript)

(fn SpawnPages
  (bind _returnvalue (Transformation|GetActorTransform))
  (Variables|Default|SetCurrentPage 0)
  (Utilities|Array|Clear (Variables|Default|GetPages))
  (Utilities|Array|Clear (Variables|Default|GetReadPages))
  (if (Utilities|Array|IsEmpty (Variables|Default|GetBookPages))
    (return)
    (else
      (bind (_arrayindex _arrayelement) (Utilities|Array|ReverseforEachLoop (Variables|Default|GetBookPages))
        (:LoopBody
          (LocalVariables|Setindex _arrayindex)
          (bind _returnvalue_2 (Game|SpawnActorfromClass "/Game/CardTest/BP_Visuals/BP_PageVisual.BP_PageVisual_C" (Math|Transform|MakeTransform (+ (.location _returnvalue) (Math|Transform|TransformDirection (Transformation|GetActorTransform) (* (Variables|Default|GetPageThickness) (- (Utilities|Array|Length (Variables|Default|GetBookPages)) (+ (LocalVariables|Getindex) 1))))) (.rotation _returnvalue) (.scale _returnvalue)) "Undefined" "MultiplyWithRoot" 0 _arrayelement 0))
          (Utilities|Array|Insert (Variables|Default|GetPages) _returnvalue_2))
        (:Completed
          (CallFunction|UpdateCurrentPages)
          (return))))))

(fn UpdateCurrentPages
  (bind _pages (Variables|Default|GetPages))
  (bind _readpages (Variables|Default|GetReadPages))
  (Utilities|FlowControl|Sequence
    (:then_0
      (if (Utilities|Array|IsEmpty _pages)
        (Variables|Default|SetCurrentPage 0)
        (else
          (Variables|Default|SetCurrentPage (Utilities|Array|Get(acopy) _pages)))))
    (:then_1
      (if (Utilities|Array|IsEmpty _readpages)
        (Variables|Default|SetCurrentReadPage 0)
        (else
          (Variables|Default|SetCurrentReadPage (Utilities|Array|Get(acopy) _readpages (Utilities|Array|LastIndex (Variables|Default|GetReadPages)))))))))

(fn ComputeNextReadPageTransform
  (bind _returnvalue (Transformation|GetActorTransform))
  (bind _readpages (Variables|Default|GetReadPages))
  (bind (_location _rotation _scale) (Math|Transform|BreakTransform _returnvalue))
  (if (Utilities|Array|IsEmpty (Variables|Default|GetReadPages))
    (return (Math|Transform|MakeTransform (+ _location (Math|Transform|TransformDirection _returnvalue (Variables|Default|GetReadPagesBaseRelativePosition))) (Math|Transform|TransformRotation _returnvalue "0.000000,179.990000,0.000000") _scale))
    (else
      (LocalVariables|SetLastReadPage (Utilities|Array|Get(acopy) _readpages (Utilities|Array|LastIndex _readpages)))
      (return (Math|Transform|MakeTransform (+ (.Location (Math|Transform|BreakTransform (Transformation|GetActorTransform (LocalVariables|GetLastReadPage)))) (Math|Transform|TransformDirection (Transformation|GetActorTransform (LocalVariables|GetLastReadPage)) (* (Variables|Default|GetPageThickness) -1.0))) (.Rotation (Math|Transform|BreakTransform (Transformation|GetActorTransform (LocalVariables|GetLastReadPage)))) (.Scale (Math|Transform|BreakTransform (Transformation|GetActorTransform (LocalVariables|GetLastReadPage)))))))))

(fn ComputeNextCurrentPageTransform
  (bind _currentpage (Variables|Default|GetCurrentPage))
  (bind _returnvalue (Transformation|GetActorTransform _currentpage))
  (bind (_location _rotation _scale) (Math|Transform|BreakTransform _returnvalue))
  (if (Utilities|Array|IsEmpty (Variables|Default|GetPages))
    (return (Transformation|GetActorTransform))
    (else
      (return (Math|Transform|MakeTransform (+ _location (Math|Transform|TransformDirection _returnvalue (Variables|Default|GetPageThickness))) _rotation _scale)))))