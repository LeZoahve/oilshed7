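; BP_AnimatedShape is a spell component actor that shows a colored mesh animating from an origin transform to a target transform.
; Init applies the given mesh, material on every slot, and a Color parameter.
; On BeginPlay a timeline lerps between the two transforms with an added height offset curve, then the actor destroys itself shortly after it finishes.
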(event EventBeginPlay
  (Utilities|Init)
  (bind (_direction _alpha _height) (Timeline|Timeline_PlayAnimation Play)
    (:Update
      (Transformation|SetActorTransform (Math|Transform|MakeTransform (+ (.location (Math|Transform|Lerp(Transform) (Variables|Default|GetOriginTransform) (Variables|Default|GetTargetTransform) _alpha)) (Math|Vector|MakeVector 0.0 0.0 _height)) (.rotation (Math|Transform|Lerp(Transform) (Variables|Default|GetOriginTransform) (Variables|Default|GetTargetTransform) _alpha)) (.scale (Math|Transform|Lerp(Transform) (Variables|Default|GetOriginTransform) (Variables|Default|GetTargetTransform) _alpha)))))
    (:Finished
      (Utilities|FlowControl|Delay 0.2)
      (Actor|DestroyActor))))

(fn ConstructionScript)